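; Enemy gameplay ability that summons random minions around its avatar.
; On activation it shuffles the computed spawn locations, plays a ground Niagara effect at each, and runs a summon montage.
; The montage's gameplay event starts a delayed loop that spawns minions one by one, slightly raised and facing the summoner.
; Each spawn increments the summoner's minion count through an interface message, and its destruction decrements it.
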(event Custom|OnDestroyed_事件
  (params (DestroyedActor :type Actor%20Object%20Reference))
  (Class|CombatInterface|IncrementMinionCount(Message) (Ability|GetAvatarActorfromActorInfo) -1))

(event Ability|EventActivateAbility
  (bind _returnvalue (Class|HeroSummonAbility|GetSpawnLocation))
  (bind _output_get (Variables|Default|SetSpawnLocations _returnvalue))
  (Utilities|Array|Shuffle _output_get)
  (for _array_element _output_get
    (Niagara|SpawnSystematLocation "/Game/Assets/Effects/Combat/NS_GroundSummon1.NS_GroundSummon1" _array_element))
  (|PlayMontageandWaitProxy "None" "/Game/SkeletonCrew/Skeleton_Mage/Animations/AM_SKM_Summon.AM_SKM_Summon" 1.0 "None" true 1.0 0.0 false
    (:then
      (Ability|Tasks|WaitGameplayEvent "(TagName=\"Montage.Attack.1\")" 0 true
        (:EventReceived
          (if (< (Variables|Default|GetSpawnLocationIndex) (Utilities|Array|Length (Variables|Default|GetSpawnLocations))) :!label _label
            (bind _returnvalue_2 (Game|SpawnActorfromClass (Class|HeroSummonAbility|GetRandomMinionClass) (Math|Transform|MakeTransform (+ (Utilities|Array|Get(acopy) (Variables|Default|GetSpawnLocations) (Variables|Default|GetSpawnLocationIndex)) "0.000000,0.000000,80.000000") (Math|Rotator|FindLookatRotation (+ (Utilities|Array|Get(acopy) (Variables|Default|GetSpawnLocations) (Variables|Default|GetSpawnLocationIndex)) "0.000000,0.000000,80.000000") (Transformation|GetActorLocation (Ability|GetAvatarActorfromActorInfo))) "1.000000,1.000000,1.000000") "AdjustIfPossibleButAlwaysSpawn" "MultiplyWithRoot" 0 0))
            (Game|AssignOnDestroyed _returnvalue_2 (delegate Custom|OnDestroyed_事件))
            (Class|CombatInterface|IncrementMinionCount(Message) (Ability|GetAvatarActorfromActorInfo) 1)
            (Math|Integer|IncrementInt (Variables|Default|GetSpawnLocationIndex)
              (:%20%20
                (Utilities|FlowControl|Delay 0.2)
                (goto _label)))))))))

(event Ability|EventOnEndAbility
  (params (bWasCancelled :type Boolean)))