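; BP_SlingshotRock is a rock actor for an enemy slingshot ability that tumbles as it exists in the world.
; BeginPlay picks random yaw, pitch and roll rates, and Tick applies them to RockMesh as frame-rate-independent local rotation.
; BeginPlay also switches the Sphere component to query-only collision after a short delay.
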(event EventBeginPlay
  (bind _returnvalue (Math|Random|RandomFloatinRange -3.6e+02 3.6e+02))
  (Variables|Default|SetYRotationRate _returnvalue)
  (Variables|Default|SetPRotationRate _returnvalue)
  (Variables|Default|SetRRotationRate _returnvalue)
  (Utilities|FlowControl|Delay 0.1)
  (Collision|SetCollisionEnabled (Variables|Default|GetSphere) "QueryOnly"))

(event EventTick
  (params (DeltaSeconds :type Float%20%28single-precision%29))
  (Transformation|AddLocalRotation (Variables|Default|GetRockMesh) (Math|Rotator|MakeRotator (* DeltaSeconds (Variables|Default|GetRRotationRate)) (* DeltaSeconds (Variables|Default|GetPRotationRate)) (* DeltaSeconds (Variables|Default|GetYRotationRate))) false false))

(fn ConstructionScript)