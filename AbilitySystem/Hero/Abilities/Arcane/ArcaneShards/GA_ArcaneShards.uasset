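; Hero arcane ability that shows a magic circle, then drops a level-scaled, capped series of shards around the clicked point.
; On input press, a temporary BP_PointCollection supplies randomly rotated ground points while the avatar faces the target and plays the cast montage.
; A montage gameplay event commits cost and starts a looping timer, each shard applying radial damage with outward knockback and firing a GameplayCue.
; Cooldown commits after the last shard.
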(event Custom|SpawnShard
  (if (< (Variables|Default|GetCount) (Math|Integer|Min(Integer) (Variables|Default|GetMaxNumShards) (Ability|GetAbilityLevel)))
    (CallFunction|StoreShardSpawnLocation)
    (CallFunction|StorePlayerstoDamage)
    (for _array_element (Variables|Default|GetPlayersToDamage)
      (CallFunction|RadialDamagetoPlayer _array_element))
    (Math|Integer|IncrementInt (Variables|Default|GetCount)
      (:%20%20
        (Class|GameplayAbility|ExecuteGameplayCuewithParams "(TagName=\"GameplayCue.ArcaneShards\")" (Ability|GameplayCue|MakeGameplayCueParameters :Location (Variables|Default|GetShardSpawnLocation)))))
    (else
      (Utilities|Time|ClearandInvalidateTimerbyHandle (Variables|Default|GetShardSpawnTimer))
      (Actor|DestroyActor (Variables|Default|GetPointCollection))
      (Ability|CommitAbilityCooldown false)
      (Ability|EndAbility))))

(event Ability|EventActivateAbility
  (bind _returnvalue (Class|GameplayAbility|CheckAbilityCost))
  (if _returnvalue
    (Utilities|FlowControl|Sequence
      (:then_0
        (Class|PlayerInterface|ShowMagicCircle(Message) (Ability|GetAvatarActorfromActorInfo) 0))
      (:then_1
        (Ability|Tasks|WaitInputPress false
          (:OnPress
            ;[1 1 1] 获取鼠标下目标
            (bind _data (|TargetDataUnderMouse)
              (:ValidData
                (Variables|Default|SetMouseHitLocation (.ImpactPoint (Collision|BreakHitResult (Ability|TargetData|GetHitResultfromTargetData _data))))
                (Utilities|FlowControl|Sequence
                  (:then_0
                    ;[1 1 1] 生成点随机点
                    (bind _returnvalue_2 (Game|SpawnActorfromClass "/Game/BP/AbilitySystem/Hero/Abilities/Arcane/ArcaneShards/BP_PointCollection.BP_PointCollection_C" (Math|Transform|MakeTransform (Variables|Default|GetMouseHitLocation) "0, 0, 0" "1.000000,1.000000,1.000000") "AlwaysSpawn" "MultiplyWithRoot" 0 0))
                    (Variables|Default|SetPointCollection _returnvalue_2)
                    (Variables|Default|SetGrondPoints (Class|PointCollection|GetGroundPoints (Variables|Default|GetPointCollection) (Variables|Default|GetMouseHitLocation) (Math|Integer|Min(Integer) (Variables|Default|GetMaxNumShards) (Ability|GetAbilityLevel)) (Math|Random|RandomFloatinRange 0.0 3.6e+02))))
                  (:then_1
                    (Class|CombatInterface|UpdateFacingTarget(Message) (Ability|GetAvatarActorfromActorInfo) (Variables|Default|GetMouseHitLocation)))
                  (:then_2
                    ;[1 1 1] 播放动画等待事件
                    (|PlayMontageandWaitProxy "None" "/Game/ModularRPGHeroesPolyart/Animations/MagicWandStance/AM_Cast_ArcaneShards.AM_Cast_ArcaneShards" 1.0 "None" false 1.0 0.0 false
                      (:then
                        (Ability|Tasks|WaitGameplayEvent "(TagName=\"Abilities.Arcane.ArcaneShards\")" 0 true
                          (:EventReceived
                            ;[1 1 1] 生成第一个和后续定时器
                            (bind _returnvalue_3 (Utilities|Time|SetTimerbyEvent (delegate Custom|SpawnShard) (Variables|Default|GetShardSpawnDeltaTime) true))
                            (Variables|Default|SetShardSpawnTimer _returnvalue_3)
                            (Class|PlayerInterface|HideMagicCircle(Message) (Ability|GetAvatarActorfromActorInfo))
                            (CallFunction|SpawnShard)
                            (Ability|CommitAbilityCost false)))))))))))))))

(event Ability|EventOnEndAbility
  (params (bWasCancelled :type Boolean)))

(fn StoreShardSpawnLocation
  (Variables|Default|SetShardSpawnLocation (Transformation|GetWorldLocation (Utilities|Array|Get(acopy) (Variables|Default|GetGrondPoints) (Variables|Default|GetCount)))))

(fn StorePlayerstoDamage
  (bind _returnvalue (Ability|GetAvatarActorfromActorInfo))
  (bind _outoverlappingactors (Class|HeroAbilitySystemLibrary|GetLivePlayerWithinRadius _returnvalue (Utilities|Array|MakeArray _returnvalue) (Variables|Default|GetRadialDamageOuterRadius) (Variables|Default|GetShardSpawnLocation)))
  (Variables|Default|SetPlayersToDamage _outoverlappingactors))

(fn RadialDamagetoPlayer
  (params (TargetActor :type Actor%20Object%20Reference))
  (bind _returnvalue (Transformation|GetActorLocation TargetActor))
  (bind _shardspawnlocation (Variables|Default|GetShardSpawnLocation))
  (bind _returnvalue_2 (- _returnvalue _shardspawnlocation))
  (Class|HeroAbilitySystemLibrary|ApplyDamageEffect (Class|HeroDamageGameplayAbility|MakeDamageEffectParamsfromClassDefaults TargetActor (Variables|Default|GetShardSpawnLocation) true _returnvalue_2 true _returnvalue_2 true 35.0)))