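; Hero gameplay ability that casts Fire Bolt, launching projectiles from the weapon socket toward the target under the mouse.
; On activation it commits, gets cursor target data, turns the avatar toward the hit location and plays the cast montage.
; A montage gameplay event triggers the spawn, passing a pitch override and the hit actor as homing target.
; The ability ends when the montage completes, blends out, is interrupted or is cancelled.
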(event Ability|EventActivateAbility
  (Ability|CommitAbility)
  (bind _data (|TargetDataUnderMouse)
    (:ValidData
      (Variables|Default|SetProjectileLocation (.Location (Collision|BreakHitResult (Ability|TargetData|GetHitResultfromTargetData _data))))
      (Variables|Default|SetMouseHit%20Actor (.HitActor (Collision|BreakHitResult (Ability|TargetData|GetHitResultfromTargetData _data))))
      (Class|CombatInterface|UpdateFacingTarget(Message) (Ability|GetAvatarActorfromActorInfo) (Variables|Default|GetProjectileLocation))
      (|PlayMontageandWaitProxy "None" "/Game/ModularRPGHeroesPolyart/Animations/MagicWandStance/AM_FireBolt.AM_FireBolt" 1.0 "None" false 1.0 0.0 false
        (:then
          (Ability|Tasks|WaitGameplayEvent "(TagName=\"Event.Montage.FireBolt\")" 0
            (:EventReceived
              (Class|HeroFireBolt|SpawnProjectiles (Variables|Default|GetProjectileLocation) (GameplayTags|MakeLiteralGameplayTag "(TagName=\"CombatSocket.Weapon\")") false 45.0 (Variables|Default|GetMouseHit%20Actor)))))
        (:OnCompleted
          (Ability|EndAbility :!label _label))
        (:OnBlendOut
          (goto _label))
        (:OnInterrupted
          (goto _label))
        (:OnCancelled
          (goto _label))))))