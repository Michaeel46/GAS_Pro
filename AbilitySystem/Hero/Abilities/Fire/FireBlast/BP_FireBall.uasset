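; BP_FireBall is the projectile actor for the Fire Blast ability, flying out and back like a boomerang before exploding.
; On authority, two timelines lerp it forward by a travel distance, then home it onto the moving ReturnToActor.
; Within explode distance of that actor, it calls OnHit, applies radial damage, pitch-overridden knockback and death impulse to nearby live players except its owner, then destroys itself.
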(event EventBeginPlay)

(event Collision|EventActorBeginOverlap
  (params (OtherActor :type Actor%20Object%20Reference)))

(event EventTick
  (params (DeltaSeconds :type Float%20%28single-precision%29)))

(event EventStartOutgoingTimeline
  (bind _returnvalue (Components|GetOwner))
  (bind _explosiondamageparams (Variables|Default|GetExplosionDamageParams))
  (bind _array (Utilities|Array|MakeArray _returnvalue))
  (Networking|SwitchHasAuthority
    (:Authority
      ;[1 1 1] 存储最初和最终位置
      (Variables|Default|SetInitialLocation (Transformation|GetActorLocation))
      (Variables|Default|SetApexLocation (+ (Variables|Default|GetInitialLocation) (* (Transformation|GetActorForwardVector) (Variables|Default|GetTravelDistance))))
      (bind _outgoing (Timeline|OutgoingTimeline Play)
        (:Update
          (Transformation|SetActorLocation (Math|Vector|Lerp(Vector) (Variables|Default|GetInitialLocation) (Variables|Default|GetApexLocation) _outgoing) false false))
        (:Finished
          (bind _returning (Timeline|ReturningTimeline Play)
            (:Update
              (Transformation|SetActorLocation (Math|Vector|Lerp(Vector) (Variables|Default|GetApexLocation) (Transformation|GetActorLocation (Variables|Default|GetReturnToActor)) _returning) false false)
              (if (CallFunction|IsWithinExplodeDistance)
                (Class|HeroProjectile|OnHit)
                (Utilities|Array|Add _array _returnvalue)
                (bind _outoverlappingactors (Class|HeroAbilitySystemLibrary|GetLivePlayerWithinRadius self _array (Variables|Default|GetRadialDamageOuterRadius) (Transformation|GetActorLocation)))
                (Variables|Default|SetOverlappingPlayers _outoverlappingactors)
                (Class|HeroAbilitySystemLibrary|SetIsRadialDamageEffectParam (Variables|Default|GetExplosionDamageParams) true (Variables|Default|GetRadialDamageInnterRadius_0) (Variables|Default|GetRadialDamageOuterRadius) (Transformation|GetActorLocation))
                (for _array_element (Variables|Default|GetOverlappingPlayers)
                  (Class|HeroAbilitySystemLibrary|SetTargetEffectParamsASC (Variables|Default|GetExplosionDamageParams) (Ability|GetAbilitySystemComponent _array_element))
                  (Variables|Default|SetKnockbackDirection (- (Transformation|GetActorLocation) (Transformation|GetActorLocation _array_element)))
                  (Class|HeroAbilitySystemLibrary|SetKnockbackDirection _explosiondamageparams (CallFunction|OverrideKnockbackPitch) (Variables|Default|GetKnockbackMagnitude))
                  (Class|HeroAbilitySystemLibrary|SetDeathImpulseDirection _explosiondamageparams (Variables|Default|GetKnockbackDirection) (Variables|Default|GetDeathImpluseMagnitude))
                  (Class|HeroAbilitySystemLibrary|ApplyDamageEffect _explosiondamageparams))
                (Actor|DestroyActor)))))))))

(fn ConstructionScript)

(fn IsWithinExplodeDistance
  (return (<= (Math|Vector|VectorLength (- (Transformation|GetActorLocation) (Transformation|GetActorLocation (Variables|Default|GetReturnToActor)))) (Variables|Default|GetExplodeDistance))))

(fn OverrideKnockbackPitch
  (bind _knockbackdirection (Variables|Default|GetKnockbackDirection))
  (bind _returnvalue (Math|Rotator|MakeRotfromX _knockbackdirection))
  (return (Math|Vector|GetForwardVector (Math|Rotator|MakeRotator (.roll _returnvalue) 45.0 (.yaw _returnvalue)))))